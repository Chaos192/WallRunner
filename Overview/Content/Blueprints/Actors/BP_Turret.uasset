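; BP_Turret is a turret that switches its color when its column is moved and tints its shot effect to match.
; ChangeColor snaps the incoming alpha to an inverted 0 or 1, then a timeline blends the Alpha material parameter on Base, Top and Barrel toward it.
; Shoot runs the parent logic, then spawns a hit-effect emitter at the projectile point, colored white or black by that target alpha.
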(event EventShoot
  ;[1 1 1] Shoot and spawn emitter,then changing its color
  (|CallParentFunction)
  (bind _returnvalue (Effects|SpawnEmitteratLocation "/Game/Effects/P_HitEffect.P_HitEffect" (Transformation|GetWorldLocation (Variables|Default|GetProjectileScene)) (Transformation|GetActorRotation) "0.500000,0.500000,0.500000"))
  (Effects|Components|ParticleSystem|SetColorParameter _returnvalue "Color" (Math|Color|Lerp(LinearColor) :A "(R=1.000000,G=1.000000,B=1.000000,A=1.000000)" :Alpha (Variables|Default|GetNewAlpha))))

(event EventChangeColor
  (params (Alpha :type Float%20%28single-precision%29))
  ;[1 1 1] Change turrets color when column is being moved
  (Variables|Default|SetNewAlpha (Math|Float|SelectFloat 0.0 1.0 (> Alpha 0.5)))
  (bind _alpha (Timeline|ChangeColorLine PlayFromStart)
    (:Update
      (bind _output_get (Variables|Default|SetCurrentAlpha (Math|Float|Lerp (Variables|Default|GetCurrentAlpha) (Variables|Default|GetNewAlpha) _alpha)))
      (Rendering|Material|SetScalarParameterValueonMaterials (Variables|Default|GetBase) "Alpha" _output_get))))

(fn ConstructionScript)