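; Turret projectile Blueprint that handles the shot's color, trail and impact effects.
; ChangeColor stores an Alpha, applies it to the sphere's materials and attaches a trail particle tinted between white and black.
; On hit it calls OnHit, then spawns a similarly tinted impact emitter scaled to DamageRadius.
; A debug sphere for the damage radius remains in the graph but is disconnected.
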(event EventBeginPlay)

(event Collision|EventHit
  (params (MyComp :type Primitive%20Component%20Object%20Reference) (Other :type Actor%20Object%20Reference) (OtherComp :type Primitive%20Component%20Object%20Reference) (bSelfMoved :type Boolean) (HitLocation :type Vector :default "0, 0, 0") (HitNormal :type Vector :default "0, 0, 0") (NormalImpulse :type Vector :default "0, 0, 0") (Hit :type Hit%20Result%20Structure%20%28by%20ref%29))
  ;[1 1 1] On hit
  (Class|TurretProjectile|OnHit)
  (bind _returnvalue (Effects|SpawnEmitteratLocation "/Game/Effects/P_HitEffect.P_HitEffect" (Transformation|GetActorLocation) (Transformation|GetActorRotation) (Math|Conversions|ToVector(Float) (/ (Variables|Default|GetDamageRadius) 28.5))))
  (Effects|Components|ParticleSystem|SetColorParameter _returnvalue "Color" (Math|Color|Lerp(LinearColor) "(R=1.000000,G=1.000000,B=1.000000,A=1.000000)" "(R=0.000000,G=0.000000,B=0.000000,A=1.000000)" (Variables|Default|GetAlpha))))

(event EventChangeColor
  (params (Alpha :type Float%20%28single-precision%29))
  ;[1 1 1] Change projectiles color and spawning trail
  (bind _output_get (Variables|Default|SetAlpha Alpha))
  (Rendering|Material|SetScalarParameterValueonMaterials (Variables|MyProjectile|GetSphere) "Alpha" _output_get)
  (bind _returnvalue (Effects|SpawnEmitterAttached "/Game/Effects/P_ProjectileTrail.P_ProjectileTrail" (Variables|MyProjectile|GetCollisionComponent) "None"))
  (Effects|Components|ParticleSystem|SetColorParameter _returnvalue "Color" (Math|Color|Lerp(LinearColor) "(R=1.000000,G=1.000000,B=1.000000,A=1.000000)" "(R=0.000000,G=0.000000,B=0.000000,A=1.000000)" (Variables|Default|GetAlpha))))

(fn ConstructionScript)