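; BP_Column is an actor for a column that moves between locations and shifts color as it does.
; Separate inner and outer move events capture the current location, then lerp to a target through their own timelines.
; A color event uses a timeline to blend a stored alpha toward a target and writes it to the mesh material's "Alpha" scalar parameter.
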(event EventBeginPlay)

(event Collision|EventActorBeginOverlap
  (params (OtherActor :type Actor%20Object%20Reference)))

(event EventTick
  (params (DeltaSeconds :type Float%20%28single-precision%29)))

(event EventMoveColumnInner
  (params (Loc :type Vector :default "0, 0, 0"))
  ;[1 1 1] Move column Up/Down
  (Variables|Default|SetStartLocation (Transformation|GetActorLocation))
  (bind _alpha (Timeline|InnerLoc PlayFromStart)
    (:Update
      (Transformation|SetActorLocation (Math|Vector|Lerp(Vector) (Variables|Default|GetStartLocation) Loc _alpha) false false))))

(event EventMoveColumnOuter
  (params (Loc :type Vector :default "0, 0, 0"))
  ;[1 1 1] Move column Up/Down
  (Variables|Default|SetStartLocation (Transformation|GetActorLocation))
  (bind _alpha (Timeline|OuterLoc PlayFromStart)
    (:Update
      (Transformation|SetActorLocation (Math|Vector|Lerp(Vector) (Variables|Default|GetStartLocation) Loc _alpha) false false))))

(event EventChangeColor
  (params (alpha :type Float%20%28single-precision%29))
  ;[1 1 1] Change column color when its Z location is being changed
  (bind _alpha (Timeline|ColorAlphaLine PlayFromStart)
    (:Update
      (bind _output_get (Variables|Default|SetCurrentAlpha (Math|Float|Lerp (Variables|Default|GetCurrentAlpha) alpha _alpha)))
      (Rendering|Material|SetScalarParameterValueonMaterials (Variables|Default|GetColumnMesh) "Alpha" _output_get))))

(fn ConstructionScript)