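; A collectible key actor that changes color with column height and plays a short animation when collected.
; ChangeColor snaps the incoming alpha to 0 or 1, then a timeline blends the mesh material's Alpha parameter toward it.
; DestroyKey disables collision, then a timeline raises the key by a Z offset while setting its yaw, and destroys the actor when finished.
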(event EventDestroyKey
  ;[1 1 1] Disable keys collision and play small animation when is being collected
  (Collision|SetActorEnableCollision false)
  (Variables|Default|SetStartLoc (Transformation|GetActorLocation))
  (bind (_direction _alphaloc _yawrot) (Timeline|DestroyAnim PlayFromStart)
    (:Update
      (Transformation|SetActorLocationAndRotation (Math|Vector|Lerp(Vector) (Variables|Default|GetStartLoc) (Math|Vector|MakeVector (.x (Variables|Default|GetStartLoc)) (.y (Variables|Default|GetStartLoc)) (+ (.z (Variables|Default|GetStartLoc)) (Variables|Default|GetEndLocZOffset))) _alphaloc) (Math|Rotator|MakeRotator 0.0 0.0 _yawrot)))
    (:Finished
      (Actor|DestroyActor))))

(event EventChangeColor
  (params (Alpha :type Float%20%28single-precision%29))
  ;[1 1 1] Change key color when column Z location is being changed
  (Variables|Default|SetNewAlpha (Math|Float|SelectFloat 0.0 1.0 (> Alpha 0.5)))
  (bind _alpha (Timeline|Timeline_1 PlayFromStart)
    (:Update
      (bind _output_get (Variables|Default|SetCurrentAlpha (Math|Float|Lerp (Variables|Default|GetCurrentAlpha) (Variables|Default|GetNewAlpha) _alpha)))
      (Rendering|Material|SetScalarParameterValueonMaterials (Variables|Default|GetKeyMesh) "Alpha" _output_get))))

(fn ConstructionScript)