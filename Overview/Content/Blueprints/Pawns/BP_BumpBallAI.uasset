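; BP_BumpBallAI is an AI-controlled ball enemy that bumps the player's BP_BallCharacter on hit.
; Each tick it pitches and rolls its eyes toward the player while its cone overlaps them, keeping capsule yaw, and rotates the sphere while moving.
; Damage drives the sphere material's Alpha from lost health, and death spawns a particle effect before destroying the actor.
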(event EventBeginPlay)

(event Collision|EventActorBeginOverlap
  (params (OtherActor :type Actor%20Object%20Reference)))

(event EventTick
  (params (DeltaSeconds :type Float%20%28single-precision%29))
  (bind _returnvalue (Game|GetPlayerCharacter 0))
  (bind _returnvalue_2 (Transformation|GetActorLocation))
  (bind _eyesscene (Variables|Default|GetEyesScene))
  (bind _returnvalue_3 (Transformation|GetActorLocation _returnvalue))
  (bind _returnvalue_4 (Math|Rotator|FindLookatRotation _returnvalue_2 _returnvalue_3))
  ;[1 1 1] Rotate AI's eyes to player
  (Utilities|FlowControl|Sequence
    (:then_0
      (if (Class|BumpBallAI|IsConeOverlappingPlayer)
        (Transformation|SetWorldRotation _eyesscene (Math|Rotator|MakeRotator (.roll _returnvalue_4) (.pitch _returnvalue_4) (.yaw (Transformation|GetWorldRotation (Variables|Default|GetCapsuleComponent)))) false false)
        (else
          (Transformation|SetWorldRotation _eyesscene (Transformation|GetWorldRotation (Variables|Default|GetCapsuleComponent)) false false))))
    (:then_1
      ;[1 1 1] Rolling AI when it is moving
      (if (>= (Math|Vector|VectorLength (Transformation|GetVelocity)) 1.0)
        (bind _returnvalue_5 (Class|BallCharacterBase|GetBallRotation))
        (Transformation|SetWorldRotation (Variables|Default|GetSphere) _returnvalue_5 false false)))))

(event EventDeath
  ;[1 1 1] Spawn emitter on death
  (Effects|SpawnEmitteratLocation "/Game/Effects/P_DeathEffect.P_DeathEffect" (Transformation|GetActorLocation) (Transformation|GetActorRotation) "3.000000,3.000000,3.000000")
  (Actor|DestroyActor))

(event Game|Damage|EventAnyDamage
  (params (Damage :type Float%20%28single-precision%29) (DamageType :type Damage%20Type%20Object%20Reference) (InstigatedBy :type Controller%20Object%20Reference) (DamageCauser :type Actor%20Object%20Reference))
  (bind _health_component (Variables|Default|GetHealth%20Component))
  ;[1 1 1] Update balls color AI is being damaged
  (Rendering|Material|SetScalarParameterValueonMaterials (Variables|Default|GetSphere) "Alpha" (- 1.0 (/ (- (Variables|/Script/Overview.HealthComponent|GetCurrentHealth _health_component) Damage) (Variables|/Script/Overview.HealthComponent|GetMaxHealth _health_component)))))

(event Collision|EventHit
  (params (MyComp :type Primitive%20Component%20Object%20Reference) (Other :type Actor%20Object%20Reference) (OtherComp :type Primitive%20Component%20Object%20Reference) (bSelfMoved :type Boolean) (HitLocation :type Vector :default "0, 0, 0") (HitNormal :type Vector :default "0, 0, 0") (NormalImpulse :type Vector :default "0, 0, 0") (Hit :type Hit%20Result%20Structure%20%28by%20ref%29))
  ;[1 1 1] Bump player on hit
  (Utilities|Casting|CastToBP_BallCharacter Other)
  (Class|BumpBallAI|BumpPlayer Other))

(fn ConstructionScript)