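; Ball-shaped character that rolls its sphere mesh while moving, darkens or recolors by health lost through a material Alpha parameter, and spawns an effect on death.
; Any hit toggles the movement mode to reset the jump count.
; Jumping sphere-traces along five directions cached at BeginPlay to find a BP_Column, then spawns a jump-off effect at the impact, tinted white or black by that column's alpha.
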(event EventBeginPlay
  (bind _returnvalue (Transformation|GetActorForwardVector))
  (bind _returnvalue_2 (Transformation|GetActorRightVector))
  (bind _linetracedirections (Variables|Default|GetLineTraceDirections))
  ;[1 1 1] Create array of all needed directions for spawning emitter when jumping off column
  (Utilities|Array|Add _linetracedirections _returnvalue)
  (Utilities|Array|Add _linetracedirections (Math|Vector|NegateVector _returnvalue))
  (Utilities|Array|Add _linetracedirections _returnvalue_2)
  (Utilities|Array|Add _linetracedirections (Math|Vector|NegateVector _returnvalue_2))
  (Utilities|Array|Add _linetracedirections (Math|Vector|NegateVector (Transformation|GetActorUpVector))))

(event Collision|EventHit
  (params (MyComp :type Primitive%20Component%20Object%20Reference) (Other :type Actor%20Object%20Reference) (OtherComp :type Primitive%20Component%20Object%20Reference) (bSelfMoved :type Boolean) (HitLocation :type Vector :default "0, 0, 0") (HitNormal :type Vector :default "0, 0, 0") (NormalImpulse :type Vector :default "0, 0, 0") (Hit :type Hit%20Result%20Structure%20%28by%20ref%29))
  (bind _charactermovement (Variables|Character|GetCharacterMovement))
  ;[1 1 1] Resetting current jump count on overlap with column mesh(CurrentJumpCount is inaccessible so we reset it by updating movement mode,because variable reserts when such functions are called)
  (Variables|Default|SetMovementMode (Variables|/Script/Engine.CharacterMovementComponent|GetMovementMode _charactermovement))
  (Pawn|Components|CharacterMovement|SetMovementMode _charactermovement "MOVE_Custom" 0)
  (Pawn|Components|CharacterMovement|SetMovementMode _charactermovement (Variables|Default|GetMovementMode) 0))

(event EventTick
  (params (DeltaSeconds :type Float%20%28single-precision%29))
  ;[1 1 1] Rolling character when it is moving
  (if (>= (Math|Vector|VectorLength (Transformation|GetVelocity)) 1.0)
    (bind _returnvalue (Class|BallCharacterBase|GetBallRotation))
    (Transformation|SetWorldRotation (Variables|Default|GetSphere) _returnvalue false false)))

(event EventDeath
  ;[1 1 1] Death emitter
  (Effects|SpawnEmitteratLocation "/Game/Effects/P_DeathEffect.P_DeathEffect" (Transformation|GetActorLocation) (Transformation|GetActorRotation) "3.000000,3.000000,3.000000"))

(event Game|Damage|EventAnyDamage
  (params (Damage :type Float%20%28single-precision%29) (DamageType :type Damage%20Type%20Object%20Reference) (InstigatedBy :type Controller%20Object%20Reference) (DamageCauser :type Actor%20Object%20Reference))
  (bind _health_component (Variables|Default|GetHealth%20Component))
  ;[1 1 1] Change balls color everytime it takes damage
  (Rendering|Material|SetScalarParameterValueonMaterials (Variables|Default|GetSphere) "Alpha" (- 1.0 (/ (- (Variables|/Script/Overview.HealthComponent|GetCurrentHealth _health_component) Damage) (Variables|/Script/Overview.HealthComponent|GetMaxHealth _health_component)))))

(event EventOnJumped
  (bind _returnvalue (Transformation|GetActorLocation))
  (bind _returnvalue_2 (- (.z _returnvalue) 4e+01))
  (bind _returnvalue_3 (Math|Vector|MakeVector (.x _returnvalue) (.y _returnvalue) _returnvalue_2))
  ;[1 1 1] Spawning emitter when jumping off column
  (Utilities|FlowControl|DoOnce false :!label _label
    (:Completed
      (bind _index (Utilities|FlowControl|ForLoopwithBreak 0 (- (Utilities|Array|Length (Variables|Default|GetLineTraceDirections)) 1) :!label _label_2)
        (:LoopBody
          (Utilities|FlowControl|DoN (Utilities|Array|Length (Variables|Default|GetLineTraceDirections)) :!label _label_3
            (:Exit
              (bind _outhit (Collision|SphereTraceByChannel _returnvalue_3 (+ _returnvalue_3 (* (Utilities|Array|Get(acopy) (Variables|Default|GetLineTraceDirections) _index) 6e+01)) 1e+01 "TraceTypeQuery1" false 0 "None"))
              (if (.bBlockingHit (Collision|BreakHitResult _outhit))
                (bind _asbp_column (Utilities|Casting|CastToBP_Column (.HitActor (Collision|BreakHitResult _outhit))))
                (Variables|Default|SetHitActor _asbp_column)
                (Variables|Default|SetHitResult _outhit)
                (goto _label_2 Break)))))
        (:Completed
          (Utilities|FlowControl|Sequence
            (:then_0
              (Utilities|IsValid (Variables|Default|GetHitActor)
                (:Is%20Valid
                  (bind _returnvalue_4 (Effects|SpawnEmitteratLocation "/Game/Effects/P_JumpOffWallEffect.P_JumpOffWallEffect" (.location (Variables|Default|GetHitResult)) (Math|Conversions|RotationFromXVector (.normal (Variables|Default|GetHitResult)))))
                  (Effects|Components|ParticleSystem|SetColorParameter _returnvalue_4 "Color" (Math|Color|SelectColor "(R=1.000000,G=1.000000,B=1.000000,A=1.000000)" "(R=0.000000,G=0.000000,B=0.000000,A=1.000000)" (> (Variables|/Game/Blueprints/Actors/BP_Column.BP_Column_C|GetCurrentAlpha (Variables|Default|GetHitActor)) 0.5)))
                  (Variables|Default|SetHitActor 0))))
            (:then_1
              (goto _label_3 Reset))
            (:then_2
              (goto _label Reset))))))))

(fn ConstructionScript)