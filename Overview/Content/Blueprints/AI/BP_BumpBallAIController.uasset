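; AI controller for BumpBall that provides yaw-rotation events for the controlled pawn, including a look-around after it reaches a patrol point.
; LookAround sweeps yaw on a timeline, whose event track retargets it the opposite way by twice RotateAngle, turning only while the pawn is nearly stationary.
; RotatetoPoint uses a second timeline to lerp yaw toward a given location, preserving pitch and roll.
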(event EventBeginPlay)

(event EventTick
  (params (DeltaSeconds :type Float%20%28single-precision%29)))

(event EventLookAround
  (bind _returnvalue (Pawn|GetControlledPawn))
  (bind _returnvalue_2 (Transformation|GetActorRotation _returnvalue))
  ;[1 1 1] Looking around after reaching patrol point
  (Variables|Default|SetStartZ (.yaw (Transformation|GetActorRotation (Pawn|GetControlledPawn))))
  (Variables|Default|SetTargetZ (+ (Variables|Default|GetStartZ) (Variables|Default|GetRotateAngle)))
  (Utilities|FlowControl|Sequence
    (:then_0
      (bind _alpha (Timeline|LookingAroundTimeLine PlayFromStart)
        (:Update
          (Utilities|FlowControl|Gate false :!label _label
            (:Exit
              (if (< (Math|Vector|VectorLength (Transformation|GetVelocity (Pawn|GetControlledPawn))) 1e+01)
                (Transformation|SetActorRotation _returnvalue (Math|Rotator|MakeRotator (.roll _returnvalue_2) (.pitch _returnvalue_2) (Math|Float|Lerp (Variables|Default|GetStartZ) (Variables|Default|GetTargetZ) _alpha)))))))
        (:ChangeProperties
          (Variables|Default|SetStartZ (.yaw (Transformation|GetActorRotation (Pawn|GetControlledPawn))))
          (Variables|Default|SetTargetZ (- (Variables|Default|GetStartZ) (* (Variables|Default|GetRotateAngle) 2.0))))))
    (:then_1
      (goto _label Open))))

(event EventRotatetoPoint
  (params (Point :type Vector :default "0, 0, 0"))
  (bind _returnvalue (Pawn|GetControlledPawn))
  (bind _returnvalue_2 (Pawn|GetControlledPawn))
  (bind _returnvalue_3 (Transformation|GetActorRotation _returnvalue))
  ;[1 1 1] Rotate AI towards location
  (Variables|Default|SetStartZ (.yaw (Transformation|GetActorRotation _returnvalue_2)))
  (Variables|Default|SetTargetZ (.yaw (Math|Rotator|FindLookatRotation (Transformation|GetActorLocation _returnvalue_2) Point)))
  (bind _alpha (Timeline|Rotation PlayFromStart)
    (:Update
      (Transformation|SetActorRotation _returnvalue (Math|Rotator|MakeRotator (.roll _returnvalue_3) (.pitch _returnvalue_3) (Math|Float|Lerp (Variables|Default|GetStartZ) (Variables|Default|GetTargetZ) _alpha))))))

(fn ConstructionScript)